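; Final dungeon door Blueprint with two large leaves that stays shut until its KeyTaken flag is set by the Open_Door event.
; Interaction always plays the door sound at the actor, even while locked.
; Once unlocked, a FlipFlop alternates playing and reversing a Timeline that drives the leaves' relative yaw.
; The track value is negated for the right leaf so the two swing in opposite directions.
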(event Custom|Open_Door
  (Variables|Default|SetKey_Taken true))

(event EventBeginPlay)

(event Collision|EventActorBeginOverlap
  (params (OtherActor :type Actor%20Object%20Reference)))

(event EventTick
  (params (DeltaSeconds :type Float%20%28single-precision%29)))

(event EventInteraction
  (Audio|PlaySoundatLocation "/Game/MT_Door.MT_Door" (Transformation|GetActorLocation) "0, 0, 0" 1.0 1.0 0.0 0 0 0 0)
  (if (Variables|Default|GetKey_Taken)
    (Utilities|FlowControl|FlipFlop
      (:A
        (bind _newtrack_0 (Timeline|Timeline Play)
          (:Update
            (Transformation|SetRelativeRotation (Variables|Default|GetSM_DoorWay_Large_Door_Left) (Math|Rotator|MakeRotator 0.0 0.0 _newtrack_0) false false)
            (Transformation|SetRelativeRotation (Variables|Default|GetSM_DoorWay_Large_Door_Right) (Math|Rotator|MakeRotator 0.0 0.0 (* _newtrack_0 -1.0)) false false))))
      (:B
        (Timeline|Timeline Reverse)))))

(fn ConstructionScript)