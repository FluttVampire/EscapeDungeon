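; Interactive cell door for the medieval dungeon that swings open or closed each time its Interaction event fires.
; Each interaction plays the door sound at the actor's location, and a FlipFlop alternately plays or reverses the OpenClose timeline.
; The timeline drives the door mesh's relative yaw, setting it to the track value and then immediately to its negation.
; The ToggleDoor function is an empty stub.
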(event Collision|EventActorBeginOverlap
  (params (OtherActor :type Actor%20Object%20Reference)))

(event EventTick
  (params (DeltaSeconds :type Float%20%28single-precision%29)))

(event EventInteraction
  (Audio|PlaySoundatLocation "/Game/MT_Cell_Door.MT_Cell_Door" (Transformation|GetActorLocation) "0, 0, 0" 1.0 1.0 0.0 0 0 0 0)
  (Utilities|FlowControl|FlipFlop
    (:A
      (bind _newtrack_0 (Timeline|Open/Close Play)
        (:Update
          (Transformation|SetRelativeRotation (Variables|Default|GetSM_Cell_Door) (Math|Rotator|MakeRotator 0.0 0.0 _newtrack_0) false false)
          (Transformation|SetRelativeRotation (Variables|Default|GetSM_Cell_Door) (Math|Rotator|MakeRotator 0.0 0.0 (* _newtrack_0 -1.0)) false false))))
    (:B
      (Timeline|Open/Close Reverse))))

(fn ConstructionScript)

(fn ToggleDoor
  (if true
    _))